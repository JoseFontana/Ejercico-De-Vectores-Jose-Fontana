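; Summoning system Blueprint that periodically spawns one of three creature types at random.
; On BeginPlay it starts a looping timer set by TiempodeSpaw and draws a long-lived debug sphere at its location.
; Each Spaw event rolls and prints a random number that selects the creature class.
; It also randomizes Vida and zeroes VelocidaddeMoviento, though neither visibly feeds the spawn calls.
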(event `self.ReceiveBeginPlay`
  (`KismetSystemLibrary.K2_SetTimerDelegate` (delegate `Spaw`) (`self.TiempodeSpaw`) true)
  (`KismetSystemLibrary.DrawDebugSphere` (`self.K2_GetActorLocation`) 100.0 12 (struct :`R` 1.0 :`G` 1.0 :`B` 1.0 :`A` 1.0) 3600.0 10.0))

(event `Spaw`
  (set `self.NumeroRando` (`KismetMathLibrary.RandomIntegerInRange` 1 3))
  (`KismetSystemLibrary.PrintString` (`KismetStringLibrary.Conv_IntToString` (`self.NumeroRando`)))
  (set `self.Vida` (`KismetMathLibrary.RandomFloatInRange` 1.0 5.0))
  (set `self.VelocidaddeMoviento` (0.0 0.0 0.0))
  (if (== (`self.NumeroRando`) 1)
    (`|SpawnActorFromClass` "/Game/BluePrints/EjercicoSPAW/BP_Criatura1.BP_Criatura1_C" (`KismetMathLibrary.MakeTransform` (0.0 0.0 0.0)) "Undefined" "MultiplyWithRoot" null (0.0 0.0 0.0) 0.0 null)
    (elif (== (`self.NumeroRando`) 2)
      (`|SpawnActorFromClass` "/Game/BluePrints/EjercicoSPAW/BP_Criatura2.BP_Criatura2_C" (`KismetMathLibrary.MakeTransform` (0.0 0.0 0.0)) "Undefined" "MultiplyWithRoot" null (0.0 0.0 0.0) 0.0 null)
      (elif (== (`self.NumeroRando`) 3)
        (`|SpawnActorFromClass` "/Game/BluePrints/EjercicoSPAW/BP_Criatura3.BP_Criatura3_C" (`KismetMathLibrary.MakeTransform` (0.0 0.0 0.0)) "Undefined" "MultiplyWithRoot" null (0.0 0.0 0.0) 0.0 null)))))

(fn `UserConstructionScript`)